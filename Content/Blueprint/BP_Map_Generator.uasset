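; BP_Map_Generator is a Blueprint that builds a grid of static mesh components as a procedural map.
; Its Construction Script loops over X by Y cells, spacing each mesh by Scale times 100 units plus a Space gap.
; Each mesh gets uniform scale, a random height up to HeightVariation and random rotation on all axes within RotationVariation.
; The randomness is unseeded, so the layout changes whenever the script reruns.
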(fn `UserConstructionScript`
  (bind _rotationvariation (`self.RotationVariation`))
  (bind _returnvalue (- 0.0 _rotationvariation))
  (bind _returnvalue_2 (* (`self.Scale`) 100.0))
  (for _index (range (`self.X`))
    (for _index_2 (range (`self.Y`))
      (`AddComponent|StaticMeshComponent_46` :`RelativeTransform` (`KismetMathLibrary.MakeTransform` (`KismetMathLibrary.MakeVector` (+ (* _index _returnvalue_2) (* _index (`self.Space`))) (+ (* _index_2 _returnvalue_2) (* _index_2 (`self.Space`))) (`KismetMathLibrary.RandomFloatInRange` 0.0 (`self.HeightVariation`))) (`KismetMathLibrary.MakeRot` (`KismetMathLibrary.RandomFloatInRange` _returnvalue _rotationvariation) (`KismetMathLibrary.RandomFloatInRange` _returnvalue _rotationvariation) (`KismetMathLibrary.RandomFloatInRange` _returnvalue _rotationvariation)) (`KismetMathLibrary.Conv_DoubleToVector` (`self.Scale`)))))))