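; Celestial body actor that orbits an optional Parent actor and can act as a light source.
; Each tick it rotates its offset from the parent by a pitch step scaled by Rotation and delta time, giving an orbit about the Y axis.
; The construction script builds a dynamic material from per-instance surface, fresnel and emissive settings and shows the point light according to EmitsLight.
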(event `self.ReceiveTick`
  (params (DeltaSeconds :type "Float (single-precision)"))
  (`/Engine/EditorBlueprintResources/StandardMacros.IsValid` (`self.Parent`)
    (:`Is Valid`
      (`self.K2_SetActorLocation` (+ (`self.K2_GetActorLocation` (`self.Parent`)) (`KismetMathLibrary.GreaterGreater_VectorRotator` (- (`self.K2_GetActorLocation`) (`self.K2_GetActorLocation` (`self.Parent`))) (`KismetMathLibrary.MakeRot` (* DeltaSeconds (`self.Rotation`)))))))))

(fn `UserConstructionScript`
  (bind _returnvalue (`PrimitiveComponent.CreateDynamicMaterialInstance` (`self.Mesh`) 0 null))
  (`MaterialInstanceDynamic.SetScalarParameterValue` _returnvalue "Roughness" (`self.Roughness`))
  (`MaterialInstanceDynamic.SetVectorParameterValue` _returnvalue "BaseColor" (`self.BaseColor`))
  (`MaterialInstanceDynamic.SetVectorParameterValue` _returnvalue "FresnelColor" (`self.FresnelColor`))
  (`MaterialInstanceDynamic.SetVectorParameterValue` _returnvalue "EmissiveColor" (`self.EmissiveColor`))
  (`MaterialInstanceDynamic.SetScalarParameterValue` _returnvalue "EmissiveAlpha" (`self.EmissiveAlpha`))
  (`SceneComponent.SetVisibility` (`self.PointLight`) (`self.EmitsLight`) false))