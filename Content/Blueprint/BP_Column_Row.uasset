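; BP_Column_Row is a construction-time placement Blueprint that builds a straight row of static mesh columns toward an EndPoint offset.
; When EndPoint has a nonzero X, the construction script adds meshes under the Column component every 60 units along its local X, their count set by the vector's length.
; It aims the row by rotating Column with a look-at rotation toward the actor location plus EndPoint.
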(fn `UserConstructionScript`
  (bind _returnvalue (`self.K2_GetActorLocation`))
  (bind _column (`self.Column`))
  (if (!= (* (`self.EndPoint`) (1.0 0.0 0.0)) (0.0 0.0 0.0) :`ErrorTolerance` 0.0)
    (for _index (range 1 (+ (`KismetMathLibrary.FFloor` (/ (`KismetMathLibrary.VSize` (`self.EndPoint`)) 60.0)) 1))
      (bind _returnvalue_2 (`AddComponent|StaticMeshComponent_48433` :`bManualAttachment` true))
      (`SceneComponent.K2_AttachTo` _returnvalue_2 _column "None" "KeepRelativeOffset" true)
      (`SceneComponent.K2_SetRelativeLocation` _returnvalue_2 (`KismetMathLibrary.MakeVector` (* _index 60.0)) false)
      (`SceneComponent.K2_SetRelativeRotation` _column (`KismetMathLibrary.FindLookAtRotation` _returnvalue (+ _returnvalue (`self.EndPoint`))) false))))